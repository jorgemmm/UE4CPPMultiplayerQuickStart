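; BP_QSCharacter is a character Blueprint that keeps a health bar on its Widget component up to date.
; BeginPlay prints a debug greeting and starts a looping half-second timer that calls UpdateInfo by name, so Tick is not used.
; UpdateInfo casts the component's user widget to WBP_Health and sets its BarHealth percent to current health divided by max health.
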(event `self.ReceiveBeginPlay`
  (`KismetSystemLibrary.PrintString` "Hello")
  (`KismetSystemLibrary.K2_SetTimer` null "UpdateInfo" 0.5 true))

(event `UpdateInfo`
  (bind _aswbp_health (cast `/Game/UI/WBP_Health` (`WidgetComponent.GetUserWidgetObject` (`self.Widget`))))
  (`ProgressBar.SetPercent` (`/Game/UI/WBP_Health.Bar_Health` _aswbp_health) (/ (`self.GetCurrentHealth`) (`self.GetMaxHealth`))))

(fn `UserConstructionScript`)