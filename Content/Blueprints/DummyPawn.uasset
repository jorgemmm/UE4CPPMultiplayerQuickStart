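; DummyPawn is a test-target pawn that tracks a Health value and shows it when damaged.
; AnyDamage and PointDamage both feed CalculeHealth, which subtracts the damage and clamps Health to a fixed range, so point hits are subtracted twice.
; AnyDamage also draws a temporary debug sphere and the remaining Health as debug text at the pawn's location.
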(event `self.ReceiveAnyDamage`
  (params (Damage :type "Float (single-precision)") (DamageType :type "DamageType Object Reference") (InstigatedBy :type "Controller Object Reference") (DamageCauser :type "Actor Object Reference"))
  (bind _returnvalue (`self.K2_GetActorLocation`))
  (`self.CalculeHealth` Damage)
  (`KismetSystemLibrary.DrawDebugSphere` _returnvalue 25.0 12 (struct :`R` 1.0 :`G` 0.682821 :`B` 0.022305 :`A` 1.0) 2.0 1.0)
  (`KismetSystemLibrary.DrawDebugString` _returnvalue (`KismetStringLibrary.Conv_DoubleToString` (`self.Health`)) null (struct :`R` 1.0 :`G` 1.0 :`B` 1.0 :`A` 1.0) 3.0))

(event `self.ReceivePointDamage`
  (params (Damage :type "Float (single-precision)") (DamageType :type "DamageType Object Reference") (HitLocation :type "Vector Structure") (HitNormal :type "Vector Structure") (HitComponent :type "PrimitiveComponent Object Reference") (BoneName :type Name) (ShotFromDirection :type "Vector Structure") (InstigatedBy :type "Controller Object Reference") (DamageCauser :type "Actor Object Reference") (HitInfo :type "HitResult Structure (by ref)"))
  (`self.CalculeHealth` Damage))

(fn `CalculeHealth`
  (params (DeltaDamage :type "Float (double-precision)"))
  (set `self.Health` (`KismetMathLibrary.FClamp` (- (`self.Health`) DeltaDamage) 0.0 100.0))
  (return))

(fn `UserConstructionScript`)